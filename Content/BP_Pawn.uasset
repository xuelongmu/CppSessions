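; Player pawn that spawns and removes BP_Spawnable cylinders with the 1 and 2 keys.
; Key 1 passes a point 200 units ahead of the eye viewpoint to S_SpawnCylinder, which spawns the actor and appends it to LastSpawnable.
; Key 2 calls S_RemoveCylinder, which destroys the newest entry and pops it, stack-style, without an empty-array check.
; Both S_ events change the world only with authority.
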(event `Key|Two`
  (params (Key :type "Key Structure"))
  (:`Pressed`
    (`self.S_RemoveCylinder`)))

(event `Key|One`
  (params (Key :type "Key Structure"))
  (bind (_outlocation _outrotation) (`self.GetActorEyesViewPoint`))
  (:`Pressed`
    (`self.S_SpawnCylinder` (`KismetMathLibrary.MakeTransform` (+ (* (`KismetMathLibrary.GetForwardVector` _outrotation) 200.0) _outlocation)))))

(event `S_SpawnCylinder`
  (params (SpawnTransform :type "Transform Structure"))
  (`/Engine/EditorBlueprintResources/ActorMacros.Switch Has Authority`
    (:`Authority`
      (bind _returnvalue (`|SpawnActorFromClass` "/Game/BP_Spawnable.BP_Spawnable_C" SpawnTransform "Undefined" "OverrideRootScale" null null))
      (`KismetArrayLibrary.Array_Add` (`self.LastSpawnable`) _returnvalue))))

(event `S_RemoveCylinder`
  (bind _lastspawnable (`self.LastSpawnable`))
  (bind _returnvalue (`KismetArrayLibrary.Array_LastIndex` _lastspawnable))
  (`/Engine/EditorBlueprintResources/ActorMacros.Switch Has Authority`
    (:`Authority`
      (`self.K2_DestroyActor` (`|GetArrayItem` _lastspawnable _returnvalue))
      (`KismetArrayLibrary.Array_Remove` _lastspawnable _returnvalue))))

(fn `UserConstructionScript`)